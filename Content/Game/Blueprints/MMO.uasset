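; MMO Blueprint that populates the world with server-stored objects by spawning Mob0001 AI on the authority at BeginPlay.
; Send Request POSTs to the Objects/getObjects JSON endpoint, and its completion handler only returns.
; BeginPlay then immediately loops over the response's ObjectsArray, without explicitly waiting for completion, switching on each Name.
; GetTransformOfObject reads JSON transform fields, with location and rotation feeding the spawn.
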(event `self.ReceiveBeginPlay`
  (`/Engine/EditorBlueprintResources/ActorMacros.Switch Has Authority`
    (:`Authority`
      (bind _output_get (set `self.Request` (`VaRestRequestJSON.ConstructRequestExt` "POST" "json")))
      (`VaRestRequestJSON.SetRequestObject` _output_get (`VaRestJsonObject.ConstructJsonObject`))
      (add `VaRestRequestJSON.OnRequestComplete` _output_get (delegate `OnRequestComplete`))
      (`VaRestRequestJSON.ProcessURL` _output_get (`KismetStringLibrary.Concat_StrStr` (`.JSONAddress_4_CDFCA70C45177F9734C55CB411942BCC` (break `/Game/Game/Blueprints/JSONAddress` (`self.temp`))) "Objects/getObjects")))))

(event `OnRequestComplete`
  (params (Request :type "VaRestRequestJSON Object Reference"))
  (bind _returnvalue (`VaRestRequestJSON.GetResponseObject` (`self.Request`)))
  (bind _returnvalue_2 (`VaRestJsonObject.GetObjectArrayField` _returnvalue "ObjectsArray"))
  (for _array_element _returnvalue_2
    (switch `string` (`VaRestJsonObject.GetStringField` _array_element "Name")
      (:`Mob0001`
        (`AIBlueprintHelperLibrary.SpawnAIFromClass` "/Game/Game/Maps/Objects/Mob0001.Mob0001_C" null (`KismetMathLibrary.MakeVector` (`VaRestJsonObject.GetNumberField` _array_element "LocationX") (`VaRestJsonObject.GetNumberField` _array_element "LocationY") (`VaRestJsonObject.GetNumberField` _array_element "LocationZ")) (`KismetMathLibrary.MakeRot` (`VaRestJsonObject.GetNumberField` _array_element "RotationX") (`VaRestJsonObject.GetNumberField` _array_element "RotationY") (`VaRestJsonObject.GetNumberField` _array_element "RotationZ")))))))

(fn `UserConstructionScript`)