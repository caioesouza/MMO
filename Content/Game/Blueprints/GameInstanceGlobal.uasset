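; Game instance that holds the player character's data: account and character IDs, name, skin color, attributes and location.
; GetCharacterJSONRequest fills these variables from a JSON request's response object, truncating the two IDs to integers.
; GetCharacterFromGlobalInstance casts the current game instance to GameInstanceGlobal and returns all the stored fields as separate outputs.
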(fn `getCharacterFromGlobalInstance`
  (returns (IdAccount :type Integer) (IdCharacter :type Integer) (CharacterName :type String) (CharacterSkinColor :type String) (CharacterIntelligence :type "Float (double-precision)") (CharacterAgility :type "Float (double-precision)") (CharacterStrenght :type "Float (double-precision)") (CharacterResistance :type "Float (double-precision)") (CharacterStamina :type "Float (double-precision)") (CharacterLocationX :type "Float (double-precision)") (CharacterLocationY :type "Float (double-precision)") (CharacterLocationZ :type "Float (double-precision)"))
  ;[1 1 1] Get information of character from GlobalInstance
  (bind _asgame_instance_global (cast `/Game/Game/Blueprints/GameInstanceGlobal` (`GameplayStatics.GetGameInstance`))
    (:`then`
      _)
    (:`CastFailed`
      _))
  (return (`/Game/Game/Blueprints/GameInstanceGlobal.IdAccount` _asgame_instance_global) (`/Game/Game/Blueprints/GameInstanceGlobal.IdCharacter` _asgame_instance_global) (`/Game/Game/Blueprints/GameInstanceGlobal.CharacterName` _asgame_instance_global) (`/Game/Game/Blueprints/GameInstanceGlobal.CharacterSkinColor` _asgame_instance_global) (`/Game/Game/Blueprints/GameInstanceGlobal.CharacterIntelligence` _asgame_instance_global) (`/Game/Game/Blueprints/GameInstanceGlobal.CharacterAgility` _asgame_instance_global) (`/Game/Game/Blueprints/GameInstanceGlobal.CharacterStrenght` _asgame_instance_global) (`/Game/Game/Blueprints/GameInstanceGlobal.CharacterResistance` _asgame_instance_global) (`/Game/Game/Blueprints/GameInstanceGlobal.CharacterStamina` _asgame_instance_global) (`/Game/Game/Blueprints/GameInstanceGlobal.CharacterLocationX` _asgame_instance_global) (`/Game/Game/Blueprints/GameInstanceGlobal.CharacterLocationY` _asgame_instance_global) (`/Game/Game/Blueprints/GameInstanceGlobal.CharacterLocationZ` _asgame_instance_global)))

(fn `getCharacterJSONRequest`
  (params (RequestObject :type "VaRestRequestJSON Object Reference"))
  (bind _returnvalue (`VaRestRequestJSON.GetResponseObject` RequestObject))
  (set `self.IdAccount` (`KismetMathLibrary.FTrunc` (`VaRestJsonObject.GetNumberField` _returnvalue "IdAccount")))
  (set `self.IdCharacter` (`KismetMathLibrary.FTrunc` (`VaRestJsonObject.GetNumberField` _returnvalue "IdCharacter")))
  (set `self.CharacterName` (`VaRestJsonObject.GetStringField` _returnvalue "CharacterName"))
  (set `self.CharacterSkinColor` (`VaRestJsonObject.GetStringField` _returnvalue "CharacterSkinColor"))
  (set `self.CharacterIntelligence` (`VaRestJsonObject.GetNumberField` _returnvalue "CharacterIntelligence"))
  (set `self.CharacterAgility` (`VaRestJsonObject.GetNumberField` _returnvalue "CharacterAgility"))
  (set `self.CharacterStrenght` (`VaRestJsonObject.GetNumberField` _returnvalue "CharacterStrenght"))
  (set `self.CharacterResistance` (`VaRestJsonObject.GetNumberField` _returnvalue "CharacterResistance"))
  (set `self.CharacterStamina` (`VaRestJsonObject.GetNumberField` _returnvalue "CharacterStamina"))
  (set `self.CharacterLocationX` (`VaRestJsonObject.GetNumberField` _returnvalue "CharacterLocationX"))
  (set `self.CharacterLocationY` (`VaRestJsonObject.GetNumberField` _returnvalue "CharacterLocationY"))
  (set `self.CharacterLocationZ` (`VaRestJsonObject.GetNumberField` _returnvalue "CharacterLocationZ")))